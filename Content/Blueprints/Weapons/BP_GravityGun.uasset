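; BP_GravityGun is a gravity gun weapon Blueprint that drives the Niagara beam effect for grabbing.
; On grab it activates the Niagara system and feeds the grab radius into its Scale Curve parameter; on release it deactivates it.
; While a grab is active, Tick moves the Beam End parameter to the current grab location.
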(event `self.ReceiveTick`
  (params (DeltaSeconds :type "Float (single-precision)"))
  (if (`self.GetGrabActive`)
    (`NiagaraComponent.SetVariableVec3` (`self.Niagara System`) "Beam End" (`self.GetGrabLocation`))))

(event `self.OnGrab`
  (`ActorComponent.Activate` (`self.Niagara System`) false)
  (`NiagaraComponent.SetVariableFloat` (`self.Niagara System`) "Scale Curve" (`self.GetGrabRadius`)))

(event `self.OnRelease`
  (`ActorComponent.Deactivate` (`self.Niagara System`)))

(fn `UserConstructionScript`)